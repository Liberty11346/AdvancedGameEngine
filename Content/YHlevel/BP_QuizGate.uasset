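; BP_QuizGate is a level actor that reveals quiz-gate text when the player reaches its trigger volumes.
; Each of its two trigger boxes responds only to BP_ThirdPersonCharacterYH and, after a short delay, makes its own set of three TextRender components visible.
; The Blueprint has no logic to hide the text again or check answers.
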(event `self.TriggerBox.OnComponentBeginOverlap`
  (params (OverlappedComponent :type "PrimitiveComponent Object Reference") (OtherActor :type "Actor Object Reference") (OtherComp :type "PrimitiveComponent Object Reference") (OtherBodyIndex :type Integer) (bFromSweep :type Boolean) (SweepResult :type "HitResult Structure (by ref)"))
  (cast `/Game/YHlevel/BP_ThirdPersonCharacterYH` OtherActor)
  (`KismetSystemLibrary.Delay` 0.5)
  (`SceneComponent.SetVisibility` (`self.TextRender`) true false)
  (`SceneComponent.SetVisibility` (`self.TextRender1`) true false)
  (`SceneComponent.SetVisibility` (`self.TextRender2`) true false))

(event `self.TriggerBox1.OnComponentBeginOverlap`
  (params (OverlappedComponent :type "PrimitiveComponent Object Reference") (OtherActor :type "Actor Object Reference") (OtherComp :type "PrimitiveComponent Object Reference") (OtherBodyIndex :type Integer) (bFromSweep :type Boolean) (SweepResult :type "HitResult Structure (by ref)"))
  (cast `/Game/YHlevel/BP_ThirdPersonCharacterYH` OtherActor)
  (`KismetSystemLibrary.Delay` 0.5)
  (`SceneComponent.SetVisibility` (`self.TextRender3`) true false)
  (`SceneComponent.SetVisibility` (`self.TextRender4`) true false)
  (`SceneComponent.SetVisibility` (`self.TextRender5`) true false))

(fn `UserConstructionScript`)