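; BP_TrapFalling is a falling-floor trap actor that drops characters through the floor when they enter its trigger.
; On TrapTrigger overlap by a Character, it hides FloorToHide, removes its collision and spawns a scaled-up explosion emitter at the floor's location.
; It also disables collision on the trigger, so it fires only once, and on three glass components, which stay visible.
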(event `self.TrapTrigger.OnComponentBeginOverlap`
  (params (OverlappedComponent :type "PrimitiveComponent Object Reference") (OtherActor :type "Actor Object Reference") (OtherComp :type "PrimitiveComponent Object Reference") (OtherBodyIndex :type Integer) (bFromSweep :type Boolean) (SweepResult :type "HitResult Structure (by ref)"))
  (bind _floortohide (`self.FloorToHide`))
  (cast `Character` OtherActor)
  (`SceneComponent.SetVisibility` (`self.FloorToHide`) false false)
  (`PrimitiveComponent.SetCollisionEnabled` _floortohide "NoCollision")
  (`GameplayStatics.SpawnEmitterAtLocation` "/Game/StarterContent/Particles/P_Explosion.P_Explosion" (`SceneComponent.K2_GetComponentLocation` _floortohide) (struct) (5.0 5.0 5.0))
  (`PrimitiveComponent.SetCollisionEnabled` (`self.TrapTrigger`) "NoCollision")
  (`PrimitiveComponent.SetCollisionEnabled` (`self.LeftGlass`) "NoCollision")
  (`PrimitiveComponent.SetCollisionEnabled` (`self.LeftGlass1`) "NoCollision")
  (`PrimitiveComponent.SetCollisionEnabled` (`self.MiddleGlass1`) "NoCollision"))

(fn `UserConstructionScript`)