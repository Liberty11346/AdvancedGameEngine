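; BP_StartGate is a level start gate that shows a countdown and then opens when the player presses E.
; It enables input for player 0, and E, guarded by a Start flag this Blueprint never sets, calls StartGameSequence to swap the intro texts for the counter.
; Chained Delays step the count and flash StartText, then hide the Cube and disable its collision.
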(event `self.ReceiveBeginPlay`
  (`self.EnableInput` (`GameplayStatics.GetPlayerController` 0))
  (`SceneComponent.SetVisibility` (`self.StartText`) false false)
  (`SceneComponent.SetVisibility` (`self.NumberCount`) false false)
  (set `self.bWallStarted` false))

(event `Key|E` :consume false
  (params (Key :type "Key Structure"))
  (bind _numbercount (`self.NumberCount`))
  (:`Pressed`
    (if (not (`self.bStart?`))
      (`self.StartGameSequence`)
      (`KismetSystemLibrary.Delay` 1.0)
      (`TextRenderComponent.K2_SetText` _numbercount (`KismetTextLibrary.Conv_StringToText` "2"))
      (`KismetSystemLibrary.Delay` 1.0)
      (`TextRenderComponent.K2_SetText` _numbercount (`KismetTextLibrary.Conv_StringToText` "1"))
      (`KismetSystemLibrary.Delay` 1.0)
      (`SceneComponent.SetVisibility` (`self.NumberCount`) false false)
      (`SceneComponent.SetVisibility` (`self.StartText`) true false)
      (`KismetSystemLibrary.Delay` 0.3)
      (`SceneComponent.SetVisibility` (`self.StartText`) false false)
      (`SceneComponent.SetVisibility` (`self.Cube`) false false)
      (`PrimitiveComponent.SetCollisionEnabled` (`self.Cube`) "NoCollision"))))

(fn `StartGameSequence`
  (`SceneComponent.SetVisibility` (`self.Mapname`) false false)
  (`SceneComponent.SetVisibility` (`self.Move`) false false)
  (`SceneComponent.SetVisibility` (`self.Jump`) false false)
  (`SceneComponent.SetVisibility` (`self.Explain`) false false)
  (`SceneComponent.SetVisibility` (`self.PressText`) false false)
  (`SceneComponent.SetVisibility` (`self.NumberCount`) true false))

(fn `UserConstructionScript`)