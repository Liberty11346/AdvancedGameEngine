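; BP_DeathWall is a moving hazard wall that sends the player to the YHMap level on contact.
; It enables input on BeginPlay, and pressing E sets CanMove after a fixed delay, starting the wall.
; Tick then offsets it along world Y by MoveSpeed scaled by delta time, without sweeping.
; A KillBox overlap with BP_ThirdPersonCharacterYH opens YHMap by name.
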(event `self.ReceiveBeginPlay`
  (`self.EnableInput` (`GameplayStatics.GetPlayerController` 0)))

(event `Key|E`
  (params (Key :type "Key Structure"))
  (:`Pressed`
    (`KismetSystemLibrary.Delay` 4.5)
    (if (not (`self.bCanMove`))
      (set `self.bCanMove` true))))

(event `self.ReceiveTick`
  (params (DeltaSeconds :type "Float (single-precision)"))
  (if (`self.bCanMove`)
    (`self.K2_AddActorWorldOffset` (`KismetMathLibrary.MakeVector` 0.0 (* (`self.MoveSpeed`) DeltaSeconds)))))

(event `self.KillBox.OnComponentBeginOverlap`
  (params (OverlappedComponent :type "PrimitiveComponent Object Reference") (OtherActor :type "Actor Object Reference") (OtherComp :type "PrimitiveComponent Object Reference") (OtherBodyIndex :type Integer) (bFromSweep :type Boolean) (SweepResult :type "HitResult Structure (by ref)"))
  (cast `/Game/YHlevel/BP_ThirdPersonCharacterYH` OtherActor)
  (`GameplayStatics.OpenLevel` "YHMap"))

(fn `UserConstructionScript`)