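; TrapGround is a trap platform that gives way under the player.
; When the player enters its trigger, it flags them as standing on it and starts a one-shot timer with a short random delay.
; If the player is still standing there when the timer fires, the mesh starts simulating physics and the trigger is destroyed.
; Leaving the trigger clears the flag but leaves the timer running.
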(event `self.ActivatePlatform_Trigger.OnComponentBeginOverlap`
  (params (OverlappedComponent :type "PrimitiveComponent Object Reference") (OtherActor :type "Actor Object Reference") (OtherComp :type "PrimitiveComponent Object Reference") (OtherBodyIndex :type Integer) (bFromSweep :type Boolean) (SweepResult :type "HitResult Structure (by ref)"))
  (if (== OtherActor (`GameplayStatics.GetPlayerCharacter` 0))
    (set `self.Standing On Platform` true)
    (bind _returnvalue (`KismetSystemLibrary.K2_SetTimerDelegate` (delegate `Platform Breaks`) (`KismetMathLibrary.RandomFloatInRange` 1.0 3.0)))))

(event `Platform Breaks`
  (if (`self.Standing On Platform`)
    (`PrimitiveComponent.SetSimulatePhysics` (`self.Platform_SM`) true)
    (`ActorComponent.K2_DestroyComponent` (`self.ActivatePlatform_Trigger`)))
  (`KismetSystemLibrary.K2_ClearAndInvalidateTimerHandle` (stale `self.ActivatePlatform_Trigger.OnComponentBeginOverlap` _returnvalue)))

(event `self.ActivatePlatform_Trigger.OnComponentEndOverlap`
  (params (OverlappedComponent :type "PrimitiveComponent Object Reference") (OtherActor :type "Actor Object Reference") (OtherComp :type "PrimitiveComponent Object Reference") (OtherBodyIndex :type Integer))
  (if (== (`GameplayStatics.GetPlayerCharacter` 0) OtherActor)
    (set `self.Standing On Platform` false)))

(fn `UserConstructionScript`)