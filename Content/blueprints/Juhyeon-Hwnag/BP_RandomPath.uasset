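; BP_RandomPath is a path actor that reveals one randomly chosen platform out of left, center and right when the player reaches it.
; A trigger box overlap by BP_ThirdPersonCharacter passes a DoOnce, so the choice happens a single time.
; A random integer switch makes the selected platform visible and sets its collision profile to BlockAll, turning it solid.
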(event `self.TriggerBox.OnComponentBeginOverlap`
  (params (OverlappedComponent :type "PrimitiveComponent Object Reference") (OtherActor :type "Actor Object Reference") (OtherComp :type "PrimitiveComponent Object Reference") (OtherBodyIndex :type Integer) (bFromSweep :type Boolean) (SweepResult :type "HitResult Structure (by ref)"))
  (cast `/Game/blueprints/Chagmin-Lee/BP_ThirdPersonCharacter` OtherActor)
  (`/Engine/EditorBlueprintResources/StandardMacros.DoOnce` false
    (:`Completed`
      (switch `int` (`KismetMathLibrary.RandomIntegerInRange` 0 2)
        (:`0`
          (`SceneComponent.SetVisibility` (`self.Platform_L`) true false)
          (`PrimitiveComponent.SetCollisionProfileName` (`self.Platform_L`) "BlockAll" true))
        (:`1`
          (`SceneComponent.SetVisibility` (`self.Platform_C`) true false)
          (`PrimitiveComponent.SetCollisionProfileName` (`self.Platform_C`) "BlockAll" true))
        (:`2`
          (`SceneComponent.SetVisibility` (`self.Platform_R`) true false)
          (`PrimitiveComponent.SetCollisionProfileName` (`self.Platform_R`) "BlockAll" true))))))

(fn `UserConstructionScript`)