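; BP_NewRandomClimb is a four-choice guessing platform that picks one correct box at random on BeginPlay.
; Entering a box as BP_ThirdPersonCharacter records its number in CurrentStep and enables actor input, while any end overlap on a box disables it.
; Pressing F calls CheckPlatform, which moves the player to NextLocation on a match with CorrectIndex, otherwise to ResetLocation.
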(event `self.ReceiveBeginPlay`
  (set `self.CorrectIndex` (`KismetMathLibrary.RandomIntegerInRange` 1 4)))

(event `self.Box1.OnComponentBeginOverlap`
  (params (OverlappedComponent :type "PrimitiveComponent Object Reference") (OtherActor :type "Actor Object Reference") (OtherComp :type "PrimitiveComponent Object Reference") (OtherBodyIndex :type Integer) (bFromSweep :type Boolean) (SweepResult :type "HitResult Structure (by ref)"))
  (cast `/Game/blueprints/Chagmin-Lee/BP_ThirdPersonCharacter` OtherActor)
  (set `self.CurrentStep` 1)
  (`self.EnableInput` (`GameplayStatics.GetPlayerController` 0)))

(event `self.Box2.OnComponentBeginOverlap`
  (params (OverlappedComponent :type "PrimitiveComponent Object Reference") (OtherActor :type "Actor Object Reference") (OtherComp :type "PrimitiveComponent Object Reference") (OtherBodyIndex :type Integer) (bFromSweep :type Boolean) (SweepResult :type "HitResult Structure (by ref)"))
  (cast `/Game/blueprints/Chagmin-Lee/BP_ThirdPersonCharacter` OtherActor)
  (set `self.CurrentStep` 2)
  (`self.EnableInput` (`GameplayStatics.GetPlayerController` 0)))

(event `self.Box3.OnComponentBeginOverlap`
  (params (OverlappedComponent :type "PrimitiveComponent Object Reference") (OtherActor :type "Actor Object Reference") (OtherComp :type "PrimitiveComponent Object Reference") (OtherBodyIndex :type Integer) (bFromSweep :type Boolean) (SweepResult :type "HitResult Structure (by ref)"))
  (cast `/Game/blueprints/Chagmin-Lee/BP_ThirdPersonCharacter` OtherActor)
  (set `self.CurrentStep` 3)
  (`self.EnableInput` (`GameplayStatics.GetPlayerController` 0)))

(event `self.Box4.OnComponentBeginOverlap`
  (params (OverlappedComponent :type "PrimitiveComponent Object Reference") (OtherActor :type "Actor Object Reference") (OtherComp :type "PrimitiveComponent Object Reference") (OtherBodyIndex :type Integer) (bFromSweep :type Boolean) (SweepResult :type "HitResult Structure (by ref)"))
  (cast `/Game/blueprints/Chagmin-Lee/BP_ThirdPersonCharacter` OtherActor)
  (set `self.CurrentStep` 4)
  (`self.EnableInput` (`GameplayStatics.GetPlayerController` 0)))

(event `Key|F`
  (params (Key :type "Key Structure"))
  (:`Pressed`
    (`self.CheckPlatform` (`self.CurrentStep`))))

(event `self.Box1.OnComponentEndOverlap`
  (params (OverlappedComponent :type "PrimitiveComponent Object Reference") (OtherActor :type "Actor Object Reference") (OtherComp :type "PrimitiveComponent Object Reference") (OtherBodyIndex :type Integer))
  (`self.DisableInput` (`GameplayStatics.GetPlayerController` 0)))

(event `self.Box2.OnComponentEndOverlap`
  (params (OverlappedComponent :type "PrimitiveComponent Object Reference") (OtherActor :type "Actor Object Reference") (OtherComp :type "PrimitiveComponent Object Reference") (OtherBodyIndex :type Integer))
  (`self.DisableInput` (`GameplayStatics.GetPlayerController` 0)))

(event `self.Box3.OnComponentEndOverlap`
  (params (OverlappedComponent :type "PrimitiveComponent Object Reference") (OtherActor :type "Actor Object Reference") (OtherComp :type "PrimitiveComponent Object Reference") (OtherBodyIndex :type Integer))
  (`self.DisableInput` (`GameplayStatics.GetPlayerController` 0)))

(event `self.Box4.OnComponentEndOverlap`
  (params (OverlappedComponent :type "PrimitiveComponent Object Reference") (OtherActor :type "Actor Object Reference") (OtherComp :type "PrimitiveComponent Object Reference") (OtherBodyIndex :type Integer))
  (`self.DisableInput` (`GameplayStatics.GetPlayerController` 0)))

(fn `CheckPlatform`
  (params (StepIndex :type Integer))
  (bind _returnvalue (`GameplayStatics.GetPlayerCharacter` 0))
  (if (== StepIndex (`self.CorrectIndex`))
    (`self.K2_SetActorLocation` _returnvalue (`self.NextLocation`) false false)
    (else
      (`self.K2_SetActorLocation` _returnvalue (`self.ResetLocation`) false false))))

(fn `UserConstructionScript`)